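; NPC_AI is an AI controller that runs the NPC_BT behavior tree for enemy characters.
; Its perception updates write whether the BP_PlayerFighterCharacter is sensed to the CanSeePlayer blackboard key for the tree, with a debug print.
; An unwired leftover fragment casts the game mode to the player character to add score and never runs.
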(event OnTargetPerceptionUpdated(AIPerception)
  (params (Actor :type Actor%20Object%20Reference) (Stimulus :type AI%20Stimulus%20Structure))
  (bind _bsuccessfullysensed (Utilities|Struct|BreakAIStimulus Stimulus))
  (Utilities|Casting|CastToBP_PlayerFighterCharacter Actor)
  (AI|Components|Blackboard|SetValueasBool (AI|GetBlackboard 0) (Utilities|Name|MakeLiteralName "CanSeePlayer") _bsuccessfullysensed)
  (Development|PrintString (Utilities|String|ToString(Boolean) _bsuccessfullysensed) _bsuccessfullysensed))

(event EventBeginPlay
  (AI|RunBehaviorTree "/Game/Blueprints/EnemyAI/NPC_BT.NPC_BT"))

(fn ConstructionScript)