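; Zombie fighter character that damages Boss_FighterCharacter with hand hits, moving at a random max walk speed picked on BeginPlay.
; Boss overlap with the Sphere sets InRange, then after a delay arms CanTakeDamage for a short window before clearing both.
; A Hand overlap deals fixed damage to the boss when CanTakeDamage and Attack are true, then disarms it.
; Attack and InRange are not set and read here, respectively.
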(event OnComponentBeginOverlap(Sphere)
  (params (OverlappedComponent :type Primitive%20Component%20Object%20Reference) (OtherActor :type Actor%20Object%20Reference) (OtherComp :type Primitive%20Component%20Object%20Reference) (OtherBodyIndex :type Integer) (bFromSweep :type Boolean) (SweepResult :type Hit%20Result%20Structure%20%28by%20ref%29))
  (Utilities|Casting|CastToBoss_FighterCharacter OtherActor)
  (Variables|Default|SetInRange true)
  (Utilities|FlowControl|Delay 1.0)
  (Variables|Default|SetCanTakeDamage true)
  (Utilities|FlowControl|Delay 2.0)
  (Variables|Default|SetInRange false)
  (Variables|Default|SetCanTakeDamage false))

(event OnComponentBeginOverlap(hand)
  (params (OverlappedComponent :type Primitive%20Component%20Object%20Reference) (OtherActor :type Actor%20Object%20Reference) (OtherComp :type Primitive%20Component%20Object%20Reference) (OtherBodyIndex :type Integer) (bFromSweep :type Boolean) (SweepResult :type Hit%20Result%20Structure%20%28by%20ref%29))
  (bind _asboss_fighter_character (Utilities|Casting|CastToBoss_FighterCharacter OtherActor))
  (if (and (Math|Boolean|Equal(Boolean) (Variables|Default|GetCanTakeDamage) true) (Math|Boolean|Equal(Boolean) (Variables|Default|Getattack) true))
    (Class|FighterCharacter|TakeDamage _asboss_fighter_character 11.0)
    (Variables|Default|SetCanTakeDamage false)))

(event EventBeginPlay
  (Variables|/Script/Engine.CharacterMovementComponent|SetMaxWalkSpeed (Variables|Character|GetCharacterMovement) (Math|Random|RandomFloatinRange 4e+02 8e+02)))

(fn ConstructionScript
  (Variables|Default|SetInRange false)
  (Variables|Default|SetCanTakeDamage false))