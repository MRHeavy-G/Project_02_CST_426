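; BP_PlayerFighterCharacter is the player's fighter, with a punch attack and a running score total.
; The Punch input arms a Punched flag, plays an animation on the mesh and clears the flag after a one-second delay.
; While armed, hit events on the left or right sphere damage the struck FighterCharacter, the left harder, then clear the flag.
; A Score event adds the given amount to ScorePoints.
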(event OnComponentHit(RightSphere)
  (params (HitComponent :type Primitive%20Component%20Object%20Reference) (OtherActor :type Actor%20Object%20Reference) (OtherComp :type Primitive%20Component%20Object%20Reference) (NormalImpulse :type Vector :default "0, 0, 0") (Hit :type Hit%20Result%20Structure%20%28by%20ref%29))
  (if (Variables|Default|Getpunched)
    (bind _asfighter_character (Utilities|Casting|CastToFighterCharacter OtherActor))
    (Class|FighterCharacter|TakeDamage _asfighter_character 4e+01)
    (Variables|Default|Setpunched false)))

(event OnComponentHit(LeftSphere)
  (params (HitComponent :type Primitive%20Component%20Object%20Reference) (OtherActor :type Actor%20Object%20Reference) (OtherComp :type Primitive%20Component%20Object%20Reference) (NormalImpulse :type Vector :default "0, 0, 0") (Hit :type Hit%20Result%20Structure%20%28by%20ref%29))
  (if (Variables|Default|Getpunched)
    (bind _asfighter_character (Utilities|Casting|CastToFighterCharacter OtherActor))
    (Class|FighterCharacter|TakeDamage _asfighter_character 5e+01)
    (Variables|Default|Setpunched false)))

(event Custom|Score
  (params (AddScore :type Integer))
  (Variables|Default|SetScore_Points (+ AddScore (Variables|Default|GetScore_Points))))

(event EventBeginPlay)

(event Collision|EventActorBeginOverlap
  (params (OtherActor :type Actor%20Object%20Reference)))

(event EventTick
  (params (DeltaSeconds :type Float%20%28single-precision%29)))

(event Input|ActionEvents|InputActionPunch
  (params (Key :type Key%20Structure :default "None"))
  (:Pressed
    (Variables|Default|Setpunched true)
    (Components|Animation|PlayAnimation (Variables|Character|GetMesh) "/Game/Character_Dev/Old_Body/Character_Movement.Character_Movement" false)
    (Utilities|FlowControl|Delay 1.0)
    (Variables|Default|Setpunched false)))

(fn ConstructionScript)